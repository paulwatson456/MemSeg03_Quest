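; BP_Speaker_01 is an information-point speaker that, when activated, plays five sounds, treated as words, in random order, only once.
; ActivatePoints shuffles the sound list and starts a looping timer, guarded by playing and already-played flags; its start sound is still unassigned.
; Each timer tick plays the next word at the speaker's location.
; After the last, it clears the timer and notifies the BP_InformationDelivery_Observer actors found at BeginPlay.
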(event `self.ReceiveBeginPlay`
  (bind _outactors (`GameplayStatics.GetAllActorsOfClass` "/Game/Blueprints/EventManagement/BP_InformationDelivery_Observer.BP_InformationDelivery_Observer_C"))
  (set `self.SpeakerObserver` _outactors))

(event `DeliverWord`
  (bind _wordnumber (`self.WordNumber`))
  (if (<= _wordnumber 4)
    (`GameplayStatics.PlaySoundAtLocation` (`|GetArrayItem` (`self.SoundList`) _wordnumber) (`SceneComponent.K2_GetComponentLocation` (`self.DefaultSceneRoot`)) (struct) 1.0 1.0 0.0 null null null)
    (set `self.WordNumber` (+ (`self.WordNumber`) 1))
    (else
      (`self.EndWordDelivery`))))

(event `/Game/Interface/INT_ActivatePoints.ActivatePoints`
  (if (not (`self.IsPlaying?`))
    (set `self.IsPlaying?` true)
    (if (not (`self.HasBeenPlayed?`))
      (set `self.HasBeenPlayed?` true)
      ;[1 1 1] Need Start Sound
      (`GameplayStatics.SpawnSoundAttached` null (`self.Cube`) "None" (0.0 0.0 0.0) (struct) "KeepRelativeOffset" false 1.0 1.0 0.0 null null)
      (bind _output_get (set `self.SoundList` (`|MakeArray` (`self.Sound_01`) (`self.Sound_02`) (`self.Sound_03`) (`self.Sound_04`) (`self.Sound_05`))))
      (`KismetArrayLibrary.Array_Shuffle` _output_get)
      (bind _returnvalue (`KismetSystemLibrary.K2_SetTimerDelegate` (delegate `DeliverWord`) 2.0 true)))))

(event `EndWordDelivery`
  (`KismetSystemLibrary.K2_ClearAndInvalidateTimerHandle` (stale `/Game/Interface/INT_ActivatePoints.ActivatePoints` _returnvalue))
  (set `self.WordNumber` 0)
  (set `self.IsPlaying?` false)
  (`/Game/Blueprints/EventManagement/BP_InformationDelivery_Observer.InformationDeliveryComplete_Event` (`self.SpeakerObserver`)))

(fn `UserConstructionScript`)