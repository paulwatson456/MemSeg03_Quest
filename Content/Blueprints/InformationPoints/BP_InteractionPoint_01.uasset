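; BP_InteractionPoint_01 is an interaction point with a widget symbol that triggers its assigned ActivationSource through an ActivatePointsMessage call.
; GeneralInteract special-cases BP_Speaker_01 sources: it requires the point to be active and disables the button if the speaker has already played.
; Enable and disable events toggle the widget's enabled state, visibility, query collision and active flag together.
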(event `/Game/Interface/INT_GeneralInteract.General Interact`
  (bind _asbp_speaker_01 (cast `/Game/Blueprints/InformationPoints/BP_Speaker_01` (stale `self.ReceiveBeginPlay` _output_get))
    (:`then`
      (if (`self.IsActive?`)
        (if (`/Game/Blueprints/InformationPoints/BP_Speaker_01.HasBeenPlayed?` _asbp_speaker_01)
          (`self.DisableButton`)
          (else
            (message `/Game/Interface/INT_ActivatePoints.ActivatePoints` (`self.ActivationSource`))))))
    (:`CastFailed`
      (message `/Game/Interface/INT_ActivatePoints.ActivatePoints` (`self.ActivationSource`)))))

(event `self.ReceiveBeginPlay`
  (bind _output_get (set `self.ActivationSource` (`self.ActivationSource`))))

(event `DisableInteraction`
  (`Widget.SetIsEnabled` (`WidgetComponent.GetUserWidgetObject` (`self.InteractionSymbol`)) false)
  (`Widget.SetVisibility` (`WidgetComponent.GetUserWidgetObject` (`self.InteractionSymbol`)) "Hidden")
  (`PrimitiveComponent.SetCollisionEnabled` (`self.InteractionSymbol`) "NoCollision")
  (set `self.IsActive?` false))

(event `EnableInteraction`
  (`Widget.SetIsEnabled` (`WidgetComponent.GetUserWidgetObject` (`self.InteractionSymbol`)) true)
  (`Widget.SetVisibility` (`WidgetComponent.GetUserWidgetObject` (`self.InteractionSymbol`)) "Visible")
  (`PrimitiveComponent.SetCollisionEnabled` (`self.InteractionSymbol`) "QueryOnly")
  (set `self.IsActive?` true))

(event `DisableButton`
  (`Widget.SetIsEnabled` (`WidgetComponent.GetUserWidgetObject` (`self.InteractionSymbol`)) false))

(fn `UserConstructionScript`)