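; Interaction plate that shows the button on a 3D start-game menu while something overlaps it.
; On BeginPlay it casts ActivationSource to UI3D_Menu_StartGame, caches it and hides its button.
; Plate collision overlap begin and end show and hide that button, with no filter on the overlapping actor.
; PowerOn and PowerOff switch the plate's collision between query-only and disabled, while GeneralInteract is an empty stub.
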(event `/Game/Interface/INT_GeneralInteract.General Interact`)

(event `self.ReceiveBeginPlay`
  (bind _output_get (set `self.ActivationSource` (`self.ActivationSource`)))
  (bind _asui3d_menu_start_game (cast `/Game/UI/UI3D_Menu_StartGame` _output_get))
  (set `self.StartMenu` _asui3d_menu_start_game)
  (`/Game/UI/UI3D_Menu_StartGame.HideButton` (`self.StartMenu`)))

(event `PowerOff`
  (`PrimitiveComponent.SetCollisionEnabled` (`self.Plate_COL`) "NoCollision"))

(event `PowerOn`
  (`PrimitiveComponent.SetCollisionEnabled` (`self.Plate_COL`) "QueryOnly"))

(event `self.Plate_COL.OnComponentBeginOverlap`
  (params (OverlappedComponent :type "PrimitiveComponent Object Reference") (OtherActor :type "Actor Object Reference") (OtherComp :type "PrimitiveComponent Object Reference") (OtherBodyIndex :type Integer) (bFromSweep :type Boolean) (SweepResult :type "HitResult Structure (by ref)"))
  (`/Game/UI/UI3D_Menu_StartGame.ShowButton` (`self.StartMenu`)))

(event `self.Plate_COL.OnComponentEndOverlap`
  (params (OverlappedComponent :type "PrimitiveComponent Object Reference") (OtherActor :type "Actor Object Reference") (OtherComp :type "PrimitiveComponent Object Reference") (OtherBodyIndex :type Integer))
  (`/Game/UI/UI3D_Menu_StartGame.HideButton` (`self.StartMenu`)))

(fn `UserConstructionScript`)