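; Level teleporter actor that fades the player's camera and loads Map_DoubleRoom_01 when its collision component is overlapped.
; On BeginPlay it casts the player pawn to PN_FPS or, failing that, VR_Pawn, storing the reference and an IsVR flag.
; The overlap event calls CameraFadeIn on the matching pawn, then opens the hardcoded map after a short delay, without checking which actor overlapped.
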(event `self.ReceiveBeginPlay`
  (bind _returnvalue (`GameplayStatics.GetPlayerPawn` 0))
  (bind _aspn_fps (cast `/Game/Controllers/Pawns/PN_FPS` _returnvalue)
    (:`then`
      (set `self.PlayerFPS` _aspn_fps))
    (:`CastFailed`
      (bind _asvr_pawn (cast `/Game/Controllers/Pawns/VR_Pawn` _returnvalue))
      (set `self.PlayerVR` _asvr_pawn)
      (set `self.IsVR?` true))))

(event `self.TeleporterCOL.OnComponentBeginOverlap`
  (params (OverlappedComponent :type "PrimitiveComponent Object Reference") (OtherActor :type "Actor Object Reference") (OtherComp :type "PrimitiveComponent Object Reference") (OtherBodyIndex :type Integer) (bFromSweep :type Boolean) (SweepResult :type "HitResult Structure (by ref)"))
  (if (`self.IsVR?`)
    (`/Game/Controllers/Pawns/VR_Pawn.CameraFadeIn` (`self.PlayerVR`))
    (`KismetSystemLibrary.Delay` 3.0)
    (`GameplayStatics.OpenLevel` "Map_DoubleRoom_01")
    (else
      (`/Game/Controllers/Pawns/PN_FPS.CameraFadeIn` (`self.PlayerFPS`))
      (`KismetSystemLibrary.Delay` 3.0)
      (`GameplayStatics.OpenLevel` "Map_DoubleRoom_01"))))

(fn `UserConstructionScript`)