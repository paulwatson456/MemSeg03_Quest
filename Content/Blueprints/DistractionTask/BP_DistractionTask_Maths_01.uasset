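; Timed maths distraction task that shows random arithmetic questions with three answer buttons on a world widget.
; ChallengeNextSequence steps through loading, description and challenge, using chained widget fade animations.
; GeneralInteract on a hovered answer loads a new shuffled question without checking correctness, until a timer ends the challenge and calls completion.
; MathsCalc builds operands, answer and two offset decoys; its division case is never rolled.
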(event `FadeText`
  (`|PlayAnimation` (`self.UITarget`) (`/Game/Blueprints/UI/UI_MathsQuestion.Anim_AllFadeOUT` (`self.UITarget`))))

(event `ChallengeNextSequence`
  (if (`self.HasLoaded?`)
    (if (`self.DescriptionShown?`)
      (`self.Start Challenge`)
      (else
        (`self.DescribeChallenge`)))
    (else
      (`self.LoadingChallenge`))))

(event `ClearScreen`
  (for _array_element (`self.MainText`)
    (`Widget.SetRenderOpacity` _array_element 0.0)
    (for _array_element_2 (`self.AllAnswers`)
      (`Widget.SetVisibility` _array_element_2 "HitTestInvisible")
      (`Widget.SetRenderOpacity` _array_element_2 0.0))))

(event `LoadingChallenge`
  (set `self.IsLoading` true)
  (`|PlayAnimation` (`self.UITarget`) (`/Game/Blueprints/UI/UI_MathsQuestion.Anim_TxtLoading_FadeIn` (`self.UITarget`)) 0.0 3 "PingPong"
    (:`Finished`
      (set `self.HasLoaded?` true)
      (`self.ChallengeNextSequence`))))

(event `self.ReceiveBeginPlay`
  (bind _uitarget (`self.UITarget`))
  (bind _output_get (set `self.WidgetTarget` (`self.Widget_Maths Question`)))
  (bind _asui_maths_question (cast `/Game/Blueprints/UI/UI_MathsQuestion` (`WidgetComponent.GetUserWidgetObject` _output_get)))
  (set `self.UITarget` _asui_maths_question)
  (set `self.Answer01` (`/Game/Blueprints/UI/UI_MathsQuestion.BTN_Answer_01` _uitarget))
  (set `self.Answer02` (`/Game/Blueprints/UI/UI_MathsQuestion.BTN_Answer_02` _uitarget))
  (set `self.Answer03` (`/Game/Blueprints/UI/UI_MathsQuestion.BTN_Answer_03` _uitarget))
  (set `self.CalcText` (`/Game/Blueprints/UI/UI_MathsQuestion.Calculation` _uitarget))
  (set `self.LoadingTxt` (`/Game/Blueprints/UI/UI_MathsQuestion.Loading` _uitarget))
  (set `self.CompleteTxt` (`/Game/Blueprints/UI/UI_MathsQuestion.Complete` _uitarget))
  (set `self.DescriptionTxt` (`/Game/Blueprints/UI/UI_MathsQuestion.ChallengeDecription` _uitarget))
  (set `self.ChallenOverTxt` (`/Game/Blueprints/UI/UI_MathsQuestion.ChallengeOver` _uitarget))
  (set `self.AllAnswers` (`|MakeArray` (`self.Answer01`) (`self.Answer02`) (`self.Answer03`)))
  (set `self.MainText` (`|MakeArray` (`self.CalcText`) (`self.LoadingTxt`) (`self.CompleteTxt`) (`self.DescriptionTxt`) (`self.ChallenOverTxt`)))
  (bind (_number01 _number02 _numbercalc _numberanswer01 _numberanswer02 _numberanswer03) (`self.MathsCalc`))
  (set `/Game/Blueprints/UI/UI_MathsQuestion.UINumber01` _number01 (`self.UITarget`))
  (set `/Game/Blueprints/UI/UI_MathsQuestion.UINumber02` _number02 (`self.UITarget`))
  (set `/Game/Blueprints/UI/UI_MathsQuestion.UINumberCalc` _numbercalc (`self.UITarget`))
  (set `/Game/Blueprints/UI/UI_MathsQuestion.UINumberAnswer` _numberanswer01 (`self.UITarget`))
  (set `/Game/Blueprints/UI/UI_MathsQuestion.UINumberAnswerWrong01` _numberanswer02 (`self.UITarget`))
  (set `/Game/Blueprints/UI/UI_MathsQuestion.UINumberAnswerWrong02` _numberanswer03 (`self.UITarget`))
  (`self.ClearScreen`))

(event `DescribeChallenge`
  (set `self.Describing` true)
  (`|PlayAnimation` (`self.UITarget`) (`/Game/Blueprints/UI/UI_MathsQuestion.Anim_Description_FadeIn` (`self.UITarget`))
    (:`Finished`
      (`KismetSystemLibrary.Delay` 2.0)
      (`|PlayAnimation` (`self.UITarget`) (`/Game/Blueprints/UI/UI_MathsQuestion.Anim_Description_FadeIn` (`self.UITarget`)) 0.0 1 "Reverse"
        (:`Finished`
          (set `self.DescriptionShown?` true)
          (`self.ChallengeNextSequence`))))))

(event `/Game/Interface/INT_GeneralInteract.General Interact`
  (bind _uitarget (`self.UITarget`))
  (if (`self.ChallengOver?`)
    _
    (elif (or (`Widget.IsHovered` (`self.Answer01`)) (`Widget.IsHovered` (`self.Answer02`)) (`Widget.IsHovered` (`self.Answer03`)))
      (if (not (`self.AnswerSelected`))
        (set `self.AnswerSelected` true)
        (`Widget.SetVisibility` (`self.AllAnswers`) "HitTestInvisible")
        (`|PlayAnimation` _uitarget (`/Game/Blueprints/UI/UI_MathsQuestion.Anim_AllAnswer_FadeIn` _uitarget) 0.0 1 "Reverse"
          (:`Finished`
            (`|PlayAnimation` (`self.UITarget`) (`/Game/Blueprints/UI/UI_MathsQuestion.Anim_Calculation_FadeIn` (`self.UITarget`)) 0.0 1 "Reverse"
              (:`Finished`
                (bind (_number01 _number02 _numbercalc _numberanswer01 _numberanswer02 _numberanswer03) (`self.MathsCalc`))
                (bind _output_get (set `self.NumberAnswers` (`|MakeArray` _numberanswer01 _numberanswer02 _numberanswer03)))
                (`KismetArrayLibrary.Array_Shuffle` _output_get)
                (set `/Game/Blueprints/UI/UI_MathsQuestion.UINumber01` _number01 (`self.UITarget`))
                (set `/Game/Blueprints/UI/UI_MathsQuestion.UINumber02` _number02 (`self.UITarget`))
                (set `/Game/Blueprints/UI/UI_MathsQuestion.UINumberCalc` _numbercalc (`self.UITarget`))
                (set `/Game/Blueprints/UI/UI_MathsQuestion.UINumberAnswer` (`|GetArrayItem` (`self.NumberAnswers`)) (`self.UITarget`))
                (set `/Game/Blueprints/UI/UI_MathsQuestion.UINumberAnswerWrong01` (`|GetArrayItem` (`self.NumberAnswers`) 1) (`self.UITarget`))
                (set `/Game/Blueprints/UI/UI_MathsQuestion.UINumberAnswerWrong02` (`|GetArrayItem` (`self.NumberAnswers`) 2) (`self.UITarget`))
                (`|PlayAnimation` (`self.UITarget`) (`/Game/Blueprints/UI/UI_MathsQuestion.Anim_Calculation_FadeIn` (`self.UITarget`)) 0.0 1 "Forward" 2.0
                  (:`Finished`
                    (`|PlayAnimation` (`self.UITarget`) (`/Game/Blueprints/UI/UI_MathsQuestion.Anim_AllAnswer_FadeIn` (`self.UITarget`)) 0.0 1 "Forward" 2.0
                      (:`Finished`
                        (`Widget.SetVisibility` (`self.AllAnswers`) "Visible")
                        (set `self.AnswerSelected` false)))))))))))))

(event `Start Challenge`
  (`KismetSystemLibrary.K2_SetTimerDelegate` (delegate `End Challenge`) 15.0)
  (set `self.ChallengOver?` false)
  (`|PlayAnimation` (`self.UITarget`) (`/Game/Blueprints/UI/UI_MathsQuestion.Anim_Calculation_FadeIn` (`self.UITarget`))
    (:`Finished`
      (`|PlayAnimation` (`self.UITarget`) (`/Game/Blueprints/UI/UI_MathsQuestion.Anim_AllAnswer_FadeIn` (`self.UITarget`))
        (:`then`
          (for _array_element (`self.AllAnswers`)
            (`Widget.SetVisibility` _array_element "Visible")))))))

(event `End Challenge`
  (set `self.ChallengOver?` true)
  (`Widget.SetVisibility` (`self.AllAnswers`) "HitTestInvisible")
  (`|PlayAnimation` (`self.UITarget`) (`/Game/Blueprints/UI/UI_MathsQuestion.Anim_Calculation_FadeIn` (`self.UITarget`)) 0.0 1 "Reverse"
    (:`then`
      (`|PlayAnimation` (`self.UITarget`) (`/Game/Blueprints/UI/UI_MathsQuestion.Anim_AllAnswer_FadeIn` (`self.UITarget`)) 0.0 1 "Reverse"
        (:`Finished`
          (`KismetSystemLibrary.Delay` 1.0)
          (`|PlayAnimation` (`self.UITarget`) (`/Game/Blueprints/UI/UI_MathsQuestion.Anim_ChallengeOver_FadeIn` (`self.UITarget`))
            (:`Finished`
              (`KismetSystemLibrary.Delay` 2.0)
              (`|PlayAnimation` (`self.UITarget`) (`/Game/Blueprints/UI/UI_MathsQuestion.Anim_ChallengeOver_FadeIn` (`self.UITarget`)) 0.0 1 "Reverse"
                (:`Finished`
                  (`self.ClearScreen`)
                  (`self.ChallengeComplete`))))))))))

(fn `MathsCalc`
  (returns (Number01 :type Text) (Number02 :type Text) (NumberCalc :type Text) (NumberAnswer01 :type Text) (NumberAnswer02 :type Text) (NumberAnswer03 :type Text))
  (locals (Number_01 :type Integer) (Number_02 :type Integer) (CalculationAnswer :type Integer) (Number_01_Text :type Text) (Number_02_Text :type Text) (NumberCalcText :type Text) (NumberAnswerText_01 :type Text) (NumberAnswerText_02 :type Text) (NumberAnswerText_03 :type Text))
  (switch `int` (`KismetMathLibrary.RandomInteger` 3)
    (:`0`
      (set `local.Number_01` (`KismetMathLibrary.RandomInteger` 10))
      (set `local.Number_02` (`KismetMathLibrary.RandomInteger` 10))
      (set `local.CalculationAnswer` (+ (`local.Number_01`) (`local.Number_02`)))
      (set `local.Number_01_Text` (`KismetTextLibrary.Conv_IntToText` (`local.Number_01`)))
      (set `local.Number_02_Text` (`KismetTextLibrary.Conv_IntToText` (`local.Number_02`)))
      (set `local.NumberCalcText` "+")
      (set `local.NumberAnswerText_01` (`KismetTextLibrary.Conv_IntToText` (`local.CalculationAnswer`)))
      (set `local.NumberAnswerText_02` (`KismetTextLibrary.Conv_IntToText` (+ (`local.CalculationAnswer`) (`KismetMathLibrary.RandomIntegerInRange` 1 12))))
      (set `local.NumberAnswerText_03` (`KismetTextLibrary.Conv_IntToText` (- (`local.CalculationAnswer`) (`KismetMathLibrary.RandomIntegerInRange` 1 12)))))
    (:`1`
      (set `local.Number_01` (`KismetMathLibrary.RandomInteger` 10))
      (set `local.Number_02` (`KismetMathLibrary.RandomInteger` 10))
      (set `local.CalculationAnswer` (- (`local.Number_01`) (`local.Number_02`)))
      (set `local.Number_01_Text` (`KismetTextLibrary.Conv_IntToText` (`local.Number_01`)))
      (set `local.Number_02_Text` (`KismetTextLibrary.Conv_IntToText` (`local.Number_02`)))
      (set `local.NumberCalcText` "-")
      (set `local.NumberAnswerText_01` (`KismetTextLibrary.Conv_IntToText` (`local.CalculationAnswer`)))
      (set `local.NumberAnswerText_02` (`KismetTextLibrary.Conv_IntToText` (+ (`local.CalculationAnswer`) (`KismetMathLibrary.RandomIntegerInRange` 1 12))))
      (set `local.NumberAnswerText_03` (`KismetTextLibrary.Conv_IntToText` (- (`local.CalculationAnswer`) (`KismetMathLibrary.RandomIntegerInRange` 1 12)))))
    (:`2`
      (set `local.Number_01` (`KismetMathLibrary.RandomInteger` 10))
      (set `local.Number_02` (`KismetMathLibrary.RandomInteger` 10))
      (set `local.CalculationAnswer` (* (`local.Number_01`) (`local.Number_02`)))
      (set `local.Number_01_Text` (`KismetTextLibrary.Conv_IntToText` (`local.Number_01`)))
      (set `local.Number_02_Text` (`KismetTextLibrary.Conv_IntToText` (`local.Number_02`)))
      (set `local.NumberCalcText` "X")
      (set `local.NumberAnswerText_01` (`KismetTextLibrary.Conv_IntToText` (`local.CalculationAnswer`)))
      (set `local.NumberAnswerText_02` (`KismetTextLibrary.Conv_IntToText` (+ (`local.CalculationAnswer`) (`KismetMathLibrary.RandomIntegerInRange` 1 12))))
      (set `local.NumberAnswerText_03` (`KismetTextLibrary.Conv_IntToText` (- (`local.CalculationAnswer`) (`KismetMathLibrary.RandomIntegerInRange` 1 12)))))
    (:`3`
      (set `local.Number_01` (`KismetMathLibrary.RandomInteger` 10))
      (set `local.Number_02` (`KismetMathLibrary.RandomInteger` 10))
      (set `local.CalculationAnswer` (/ (`local.Number_01`) (`local.Number_02`)))
      (set `local.Number_01_Text` (`KismetTextLibrary.Conv_IntToText` (`local.Number_01`)))
      (set `local.Number_02_Text` (`KismetTextLibrary.Conv_IntToText` (`local.Number_02`)))
      (set `local.NumberCalcText` "/")
      (set `local.NumberAnswerText_01` (`KismetTextLibrary.Conv_IntToText` (`local.CalculationAnswer`)))
      (set `local.NumberAnswerText_02` (`KismetTextLibrary.Conv_IntToText` (+ (`local.CalculationAnswer`) (`KismetMathLibrary.RandomIntegerInRange` 1 12))))
      (set `local.NumberAnswerText_03` (`KismetTextLibrary.Conv_IntToText` (- (`local.CalculationAnswer`) (`KismetMathLibrary.RandomIntegerInRange` 1 12))))))
  (return (`local.Number_01_Text`) (`local.Number_02_Text`) (`local.NumberCalcText`) (`local.NumberAnswerText_01`) (`local.NumberAnswerText_02`) (`local.NumberAnswerText_03`)))

(fn `UserConstructionScript`)